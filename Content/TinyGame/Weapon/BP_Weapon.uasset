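; Data-driven weapon actor that attaches to a character's mesh socket and performs sword or bow attacks for it.
; BeginPlay loads its mesh and data from DT_Weapon, and attack start plays a riding or standard montage via the BPI_Unit riding check.
; The attack notify runs on authority only, switching on weapon type.
; Swords sphere-overlap at the hit socket to damage enemy units, while bows spawn BP_Arrow toward the attack target.
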(event `self.ReceiveBeginPlay`
  (bind _returnvalue (`|GetDataTableRow` "/Game/TinyGame/Data/DT_Weapon.DT_Weapon" (`self.Row Name`))
    (:`then`
      (bind _output_get (set `self.WeaponData` _returnvalue))
      (`StaticMeshComponent.SetStaticMesh` (`self.WeaponMesh`) (`.StaticMesh_5_19DBEE6142D7A6E2C6ECC4B2AC34C406` (break `/Game/TinyGame/Data/ST_Weapon` _output_get))))))

(fn `DoShootArrow`
  (bind _asbpi_unit (cast `/Game/TinyGame/Unit/BPI_Unit` (`self.Character`)))
  (bind _target (`/Game/TinyGame/Unit/BPI_Unit.GetAttackTarget` _asbpi_unit))
  (`/Engine/EditorBlueprintResources/StandardMacros.IsValid` _target
    (:`Is Valid`
      (`|SpawnActorFromClass` "/Game/TinyGame/Weapon/BP_Arrow.BP_Arrow_C" (`KismetMathLibrary.MakeTransform` (`SceneComponent.GetSocketLocation` (`self.WeaponMesh`) "arrow") (`self.K2_GetActorRotation`)) "Undefined" "MultiplyWithRoot" null (`self.K2_GetActorLocation` _target) (`self.Character`)))))

(fn `DoSwordAttack`
  (bind _returnvalue (`SceneComponent.GetSocketLocation` (`self.WeaponMesh`) "hit"))
  (bind _outactors (`KismetSystemLibrary.SphereOverlapActors` _returnvalue 32.0 (`|MakeArray` "ObjectTypeQuery3" :!type "EObjectTypeQuery Enum") "/Game/TinyGame/Unit/BP_Unit.BP_Unit_C" (`|MakeArray` (`self.Character`) :!type "Actor Object Reference")))
  (`KismetSystemLibrary.DrawDebugSphere` _returnvalue 16.0 36 (struct :`R` 1.0 :`A` 1.0) 5.0 1.0)
  (for _array_element _outactors
    (bind _asbp_unit (cast `/Game/TinyGame/Unit/BP_Unit` _array_element))
    (if (`/Game/TinyGame/Unit/BP_Unit.IsEnemy` _asbp_unit (`self.Character`))
      (`GameplayStatics.ApplyDamage` _asbp_unit 10.0 (`Pawn.GetController` (`self.Character`)) self))))

(fn `EventAttach`
  (params (Character :type "Character Object Reference") (SocketName :type Name))
  (returns (bResult :type Boolean))
  (bind _output_get (set `self.Character` Character))
  (bind _returnvalue (`self.K2_AttachToComponent` (`Character.Mesh` _output_get) SocketName "SnapToTarget" "SnapToTarget" "SnapToTarget"))
  (return _returnvalue))

(fn `EventAttackNotify`
  (returns (bResult :type Boolean))
  (bind (_weapondata_name _weapondata_weapontype) (break `/Game/TinyGame/Data/ST_Weapon` (`self.WeaponData`)))
  (`/Engine/EditorBlueprintResources/ActorMacros.Switch Has Authority`
    (:`Authority`
      (`|ExecutionSequence`
        (:`then_0`
          (switch `/Game/TinyGame/Data/EN_WeaponType` _weapondata_weapontype
            (:`NewEnumerator1`
              (`self.DoSwordAttack`))
            (:`NewEnumerator2`
              (`self.DoShootArrow`))))
        (:`then_1`
          (return false))))))

(fn `EventAttackStart`
  (returns (bResult :type Boolean))
  (bind (_weapondata_name _weapondata_weapontype _weapondata_staticmesh _weapondata_attackanimation _weapondata_rideattackanimation) (break `/Game/TinyGame/Data/ST_Weapon` (`self.WeaponData`)))
  (bind _character (`self.Character`)
    (:`then`
      (if (`self.IsCharRiding` _character)
        (`Character.PlayAnimMontage` _character _weapondata_rideattackanimation 1.0 "None")
        (else
          (`KismetSystemLibrary.PrintString` (`KismetSystemLibrary.GetDisplayName` _weapondata_attackanimation))
          (`Character.PlayAnimMontage` _character _weapondata_attackanimation 1.0 "None")))
      (return true))
    (:`else`
      (return false))))

(fn `IsCharRiding`
  (params (Character :type "Character Object Reference"))
  (returns (IsRiding :type Boolean))
  (bind _asbpi_unit (cast `/Game/TinyGame/Unit/BPI_Unit` Character)
    (:`then`
      (bind _isriding (`/Game/TinyGame/Unit/BPI_Unit.IsRiding` _asbpi_unit))
      (return _isriding))
    (:`CastFailed`
      (return false))))

(fn `UserConstructionScript`)