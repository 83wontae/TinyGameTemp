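; A component that gives a Character unit a viewport name tag showing its name, HP and SH values.
; On BeginPlay it creates the NameTag widget with a reference to itself, adds it to the viewport, and initializes it with the attach parent's owning Character, printing an error if the cast fails.
; Setter functions forward values to the widget, with only SetHp checking validity, and EndPlay removes it.
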(event `self.ReceiveBeginPlay`
  (bind _returnvalue (`|CreateWidget` "/Game/TinyGame/Nametag/NameTagWidget.NameTagWidget_C" null self))
  (bind _output_get (set `self.NameTag` _returnvalue))
  (`UserWidget.AddToViewport` _output_get 0)
  (bind _ascharacter (cast `Character` (`self.GetOwner` (`self.GetAttachParent`)))
    (:`then`
      (`self.InitCharacter` _ascharacter))
    (:`CastFailed`
      (`KismetSystemLibrary.PrintString` "Nametag Attach Target is not Character!!!" true true (struct :`R` 1.0 :`B` 0.008 :`A` 1.0) 30.0))))

(event `self.ReceiveEndPlay`
  (params (EndPlayReason :type "EEndPlayReason Enum" :default "Destroyed"))
  (`Widget.RemoveFromParent` (`self.NameTag`)))

(fn `InitCharacter`
  (params (Character :type "Character Object Reference"))
  (`/Game/TinyGame/Nametag/NameTagWidget.InitCharacter` (`self.NameTag`) Character))

(fn `SetHp`
  (params (CurHp :type "Float (double-precision)") (MaxHp :type "Float (double-precision)"))
  (bind _nametag (`self.NameTag`)
    (:`then`
      (`/Game/TinyGame/Nametag/NameTagWidget.SetHp` _nametag CurHp MaxHp))
    (:`else`)))

(fn `SetName`
  (params (Name :type String))
  (`/Game/TinyGame/Nametag/NameTagWidget.SetName` (`self.NameTag`) Name))

(fn `SetSH `
  (params (CurSH :type "Float (double-precision)") (MaxSH :type "Float (double-precision)"))
  (`/Game/TinyGame/Nametag/NameTagWidget.SetSH` (`self.NameTag`) CurSH MaxSH))