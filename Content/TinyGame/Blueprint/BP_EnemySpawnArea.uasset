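; Enemy spawn area actor that periodically spawns AI units while its spawning flag is on.
; Tick accumulates time toward SpawnTime, shows progress on the name tag gauge, and resets it when spawning is off.
; SpawnUnit looks up the unit class in DT_Unit, spawns it with BT_Unit at a random point on a surrounding circle, then initializes it through BPI_Unit with OverlapUnit as leader and weapon row names.
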(event `self.ReceiveTick`
  (params (DeltaSeconds :type "Float (single-precision)"))
  (if (`self.IsSpawning`)
    (bind _output_get (set `self.TotalDeltaSeconds` (+ DeltaSeconds (`self.TotalDeltaSeconds`))))
    (`/Game/TinyGame/Nametag/BP_ActorNameTagComponent.SetGauge` (`self.BP_ActorNameTagComponent`) _output_get (`self.SpawnTime`))
    (if (> (`self.TotalDeltaSeconds`) (`self.SpawnTime`))
      (`self.SpawnUnit`))
    (else
      (bind _output_get_2 (set `self.TotalDeltaSeconds` 0.0))
      (`/Game/TinyGame/Nametag/BP_ActorNameTagComponent.SetGauge` (`self.BP_ActorNameTagComponent`) _output_get_2 (`self.SpawnTime`)))))

(fn `GetRandomRoundLocation`
  (params (Radius :type "Float (double-precision)" :default 200.0))
  (returns (RandLocation :type "Vector Structure"))
  (locals (`Rand Radian` :type "Float (double-precision)"))
  (bind _rand_radian (`local.Rand Radian`))
  (set `local.Rand Radian` (`KismetMathLibrary.DegreesToRadians` (`KismetMathLibrary.RandomFloatInRange` 0.0 360.0)))
  (return (+ (`self.K2_GetActorLocation`) (`KismetMathLibrary.MakeVector` (* (`KismetMathLibrary.Cos` _rand_radian) (`local.Radius`)) (* (`KismetMathLibrary.Sin` _rand_radian) (`local.Radius`))) (0.0 0.0 80.0))))

(fn `SpawnUnit`
  (set `self.TotalDeltaSeconds` 0.0)
  (bind _returnvalue (`|GetDataTableRow` "/Game/TinyGame/Data/DT_Unit.DT_Unit" (`self.Unit Row Name`))
    (:`then`
      (bind _returnvalue_2 (`AIBlueprintHelperLibrary.SpawnAIFromClass` (`.UnitClass_35_6F6C0F764B406FFBEA7B90B1A9BC7855` (break `/Game/TinyGame/Data/ST_Unit` _returnvalue)) "/Game/TinyGame/AI/BT_Unit.BT_Unit" (`self.GetRandomRoundLocation` 200.0) (struct) true null))
      (bind _asbpi_unit (cast `/Game/TinyGame/Unit/BPI_Unit` _returnvalue_2))
      (`/Game/TinyGame/Unit/BPI_Unit.InitUnit` _asbpi_unit (`self.OverlapUnit`) (`self.Unit Row Name`) (`self.L Weapon Row Name`) (`self.R Weapon Row Name`)))))

(fn `UserConstructionScript`)