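; BP_SpawnArea is a zone that periodically spawns allied AI units while a player-controlled BP_Unit stands inside its box.
; Box overlaps toggle spawning and store that unit; Tick accumulates time, shows progress on the name tag gauge and resets it when spawning stops.
; When the timer exceeds SpawnTime, it spawns a BP_Unit with BT_Unit, initialized with configured row names and the overlapping unit as master.
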(event `self.ReceiveTick`
  (params (DeltaSeconds :type "Float (single-precision)"))
  (if (`self.IsSpawning`)
    (bind _output_get (set `self.TotalDeltaSeconds` (+ DeltaSeconds (`self.TotalDeltaSeconds`))))
    (`/Game/TinyGame/Nametag/BP_ActorNameTagComponent.SetGauge` (`self.BP_ActorNameTagComponent`) _output_get (`self.SpawnTime`))
    (if (> (`self.TotalDeltaSeconds`) (`self.SpawnTime`))
      (`self.SpawnUnit`))
    (else
      (bind _output_get_2 (set `self.TotalDeltaSeconds` 0.0))
      (`/Game/TinyGame/Nametag/BP_ActorNameTagComponent.SetGauge` (`self.BP_ActorNameTagComponent`) _output_get_2 (`self.SpawnTime`)))))

(event `self.Box.OnComponentBeginOverlap`
  (params (OverlappedComponent :type "PrimitiveComponent Object Reference") (OtherActor :type "Actor Object Reference") (OtherComp :type "PrimitiveComponent Object Reference") (OtherBodyIndex :type Integer) (bFromSweep :type Boolean) (SweepResult :type "HitResult Structure (by ref)"))
  (bind _asbp_unit (cast `/Game/TinyGame/Unit/BP_Unit` OtherActor))
  (if (`Pawn.IsPlayerControlled` _asbp_unit)
    (set `self.OverlapUnit` _asbp_unit)
    (set `self.IsSpawning` true)))

(event `self.Box.OnComponentEndOverlap`
  (params (OverlappedComponent :type "PrimitiveComponent Object Reference") (OtherActor :type "Actor Object Reference") (OtherComp :type "PrimitiveComponent Object Reference") (OtherBodyIndex :type Integer))
  (bind _asbp_unit (cast `/Game/TinyGame/Unit/BP_Unit` OtherActor))
  (if (`Pawn.IsPlayerControlled` _asbp_unit)
    (set `self.OverlapUnit` null)
    (set `self.IsSpawning` false)))

(fn `SpawnUnit`
  (set `self.TotalDeltaSeconds` 0.0)
  (bind _returnvalue (`AIBlueprintHelperLibrary.SpawnAIFromClass` "/Game/TinyGame/Unit/BP_Unit.BP_Unit_C" "/Game/TinyGame/AI/BT_Unit.BT_Unit" (`SceneComponent.K2_GetComponentLocation` (`self.BP_ActorNameTagComponent`)) (struct) true null))
  (bind _asbp_unit (cast `/Game/TinyGame/Unit/BP_Unit` _returnvalue))
  (`/Game/TinyGame/Unit/BP_Unit.InitUnit` _asbp_unit (`self.OverlapUnit`) (`self.Unit Row Name`) (`self.R Weapon Row Name`) (`self.L Weapon Row Name`)))

(fn `UserConstructionScript`)